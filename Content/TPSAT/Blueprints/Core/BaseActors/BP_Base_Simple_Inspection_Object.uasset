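; Base actor for simple inspectable objects that can play player dialogue, focus the camera and report quest interactions.
; The top-button interaction plays table-driven voice and subtitles when the dialogue row is valid.
; If camera focus is enabled, it then focuses and notifies the player's quest component.
; The right-button interaction always notifies the quest component with the object's class, then saves the game.
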(event `self.TopButtonInteraction`
  (`|ExecutionSequence`
    (:`then_0`
      (bind (_dialogue_waves _subtitles _validdata) (`/Game/TPSAT/Blueprints/Core/BP_StoryAdv_FunctionLibrary.GetDialogueDataFromTable` (`self.DialogueRow`)))
      (if _validdata
        (`/Game/TPSAT/Blueprints/Core/BP_StoryAdv_GameController.PlayPlayerDialogue` (`self.GameControllerInstance`) _dialogue_waves _subtitles)))
    (:`then_1`
      (if (`self.UseCameraFocus`)
        (`self.CameraFocus`)
        (`/Game/Vindolanda/Blueprints/Common/Quest/BP_QuestComponent.OnQuestItemIneracted` (`self.GetComponentByClass` (`GameplayStatics.GetPlayerCharacter` 0) "/Game/Vindolanda/Blueprints/Common/Quest/BP_QuestComponent.BP_QuestComponent_C") "NewEnumerator3" (`GameplayStatics.GetObjectClass` self))))))

(event `self.RightButtonInteraction`
  (`/Game/Vindolanda/Blueprints/Common/Quest/BP_QuestComponent.OnQuestItemIneracted` (`self.GetComponentByClass` (`GameplayStatics.GetPlayerCharacter` 0) "/Game/Vindolanda/Blueprints/Common/Quest/BP_QuestComponent.BP_QuestComponent_C") "NewEnumerator3" (`GameplayStatics.GetObjectClass` self))
  (`/Game/TPSAT/Blueprints/Core/BP_StoryAdv_GameInstance.SaveGame` (`/Game/TPSAT/Blueprints/Core/BP_StoryAdv_FunctionLibrary.GetStoryAdvGameInstance`) true))

(fn `UserConstructionScript`
  (`parent.UserConstructionScript`))