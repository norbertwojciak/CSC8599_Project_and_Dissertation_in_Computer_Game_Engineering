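; BP_Note is a storytelling note actor that reveals animated text on a widget component placed in the level.
; The widget starts hidden and appears once, either at BeginPlay when StartAnimation is set or when a BP_StoryAdv_Character overlaps the sphere trigger.
; On reveal it passes the text, styling and per-sign animation settings to the widget through UpdateNoteMessage.
; The construction script applies the note's transform and draw size and disables shadow casting.
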(event `self.ReceiveBeginPlay`
  (`SceneComponent.SetVisibility` (`self.Widget`) false false)
  (if (`self.bStartAnimation`)
    (if (not (`self.bVisited`)) :!label _label
      (set `self.bVisited` true)
      (`SceneComponent.SetVisibility` (`self.Widget`) true false)
      (message `/Game/Vindolanda/Blueprints/Common/Storytelling/BPI_Storytelling.UpdateNote` (`WidgetComponent.GetUserWidgetObject` (`self.Widget`)) (`self.Text`) (`self.TextColor`) (`self.Font`) (`self.DelayBetweenSigns`) (`self.WidgetSize`) (`self.SignAnimation`)))))

(event `self.Sphere.OnComponentBeginOverlap`
  (params (OverlappedComponent :type "PrimitiveComponent Object Reference") (OtherActor :type "Actor Object Reference") (OtherComp :type "PrimitiveComponent Object Reference") (OtherBodyIndex :type Integer) (bFromSweep :type Boolean) (SweepResult :type "HitResult Structure (by ref)"))
  (cast `/Game/TPSAT/Blueprints/Character/BP_StoryAdv_Character` OtherActor)
  (goto _label))

(fn `UserConstructionScript`
  (`SceneComponent.K2_SetRelativeLocationAndRotation` (`self.Widget`) (`self.NoteLocation`) (`self.NoteRotation`) false false)
  (`PrimitiveComponent.SetCastShadow` (`self.Widget`) false)
  (`WidgetComponent.SetDrawSize` (`self.Widget`) (`self.WidgetSize`)))