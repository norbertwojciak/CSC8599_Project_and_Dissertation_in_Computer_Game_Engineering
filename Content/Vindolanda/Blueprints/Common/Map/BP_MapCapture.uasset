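; Map capture actor that renders top-down world maps, with and without legend, and supplies map projection planes to the player.
; The construction script sizes cameras and planes from world size; its Capture toggle triggers one-shot orthographic captures of "Capture"-tagged actors, exporting named ones as PNGs.
; At BeginPlay, assigned map textures feed the planes' dynamic materials, and a looping timer polls for the player character to pass it both planes.
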(event `CheckPlayerAndProceed`
  (`/Engine/EditorBlueprintResources/StandardMacros.IsValid` (`GameplayStatics.GetPlayerCharacter` 0)
    (:`Is Valid`
      (`KismetSystemLibrary.K2_ClearAndInvalidateTimerHandle` (`self.CheckPlayerTimer`))
      (message `/Game/Vindolanda/Blueprints/Core/BPI_Player_Character.UpdatePlayerMap` (`GameplayStatics.GetPlayerCharacter` 0) (`self.ProjectionPlaneLegend`))
      (message `/Game/Vindolanda/Blueprints/Core/BPI_Player_Character.UpdatePlayerMap` (`GameplayStatics.GetPlayerCharacter` 0) (`self.ProjectionPlaneNoLegend`)))))

(event `self.ReceiveBeginPlay`
  ;[1 1 1] Legend
  (bind _returnvalue (`PrimitiveComponent.CreateDynamicMaterialInstance` (`self.ProjectionPlaneLegend`) 0 "/Game/Vindolanda/Materials/Map/M_MapProjectionLegend.M_MapProjectionLegend" "None"))
  (set `self.MID_MapProjectionLegend` _returnvalue)
  (`MaterialInstanceDynamic.SetTextureParameterValue` (`self.MID_MapProjectionLegend`) "TextureLegend" (`self.MapTextureLegend`))
  ;[1 1 1] No Legend
  (bind _returnvalue_2 (`PrimitiveComponent.CreateDynamicMaterialInstance` (`self.ProjectionPlaneNoLegend`) 0 "/Game/Vindolanda/Materials/Map/M_MapProjectionNoLegend.M_MapProjectionNoLegend" "None"))
  (set `self.MID_MapProjectionNoLegend` _returnvalue_2)
  (`MaterialInstanceDynamic.SetTextureParameterValue` (`self.MID_MapProjectionNoLegend`) "TextureNoLegend" (`self.MapTextureNoLegend`))
  (bind _returnvalue_3 (`KismetSystemLibrary.K2_SetTimerDelegate` (`|CreateDelegate` :!event `CheckPlayerAndProceed`) 0.2 true))
  (set `self.CheckPlayerTimer` _returnvalue_3))

(fn `MapCaptureLegend`
  (locals (RT_MapCaptureLegend :type "TextureRenderTarget2D Object Reference"))
  (bind _capturesize (`self.CaptureSize`))
  (bind _returnvalue (`KismetRenderingLibrary.CreateRenderTarget2D` _capturesize _capturesize))
  (bind _output_get (set `local.RT_MapCaptureLegend` _returnvalue))
  (set `SceneCaptureComponent2D.TextureTarget` _output_get (`self.SceneCaptureWithLegend`))
  (set `SceneCaptureComponent2D.OrthoWidth` (`self.WorldSizeInUnits`) (`self.SceneCaptureWithLegend`))
  (bind _outactors (`GameplayStatics.GetAllActorsWithTag` "Capture"))
  (set `SceneCaptureComponent.ShowOnlyActors` _outactors (`self.SceneCaptureWithLegend`))
  (`SceneCaptureComponent2D.CaptureScene` (`self.SceneCaptureWithLegend`))
  (if (`KismetStringLibrary.NotEqual_StrStr` (`self.TextureNameLegend`))
    (`KismetRenderingLibrary.ExportRenderTarget` (`local.RT_MapCaptureLegend`) (`KismetStringLibrary.Concat_StrStr` (`KismetSystemLibrary.GetProjectContentDirectory`) "Vindolanda/Maps/MapCapture") (`KismetStringLibrary.Concat_StrStr` "T_" (`self.TextureNameLegend`) ".png"))))

(fn `MapCaptureNoLegend`
  (locals (RT_MapCaptureNoLegend :type "TextureRenderTarget2D Object Reference"))
  (bind _capturesize (`self.CaptureSize`))
  (bind _returnvalue (`KismetRenderingLibrary.CreateRenderTarget2D` _capturesize _capturesize))
  (bind _output_get (set `local.RT_MapCaptureNoLegend` _returnvalue))
  (set `SceneCaptureComponent2D.TextureTarget` _output_get (`self.SceneCaptureWithNoLegend`))
  (set `SceneCaptureComponent2D.OrthoWidth` (`self.WorldSizeInUnits`) (`self.SceneCaptureWithNoLegend`))
  (bind _outactors (`GameplayStatics.GetAllActorsWithTag` "Capture"))
  (set `SceneCaptureComponent.ShowOnlyActors` _outactors (`self.SceneCaptureWithNoLegend`))
  (`SceneCaptureComponent2D.CaptureScene` (`self.SceneCaptureWithNoLegend`))
  (if (`KismetStringLibrary.NotEqual_StrStr` (`self.TextureNameNoLegend`))
    (`KismetRenderingLibrary.ExportRenderTarget` (`local.RT_MapCaptureNoLegend`) (`KismetStringLibrary.Concat_StrStr` (`KismetSystemLibrary.GetProjectContentDirectory`) "Vindolanda/Maps/MapCapture") (`KismetStringLibrary.Concat_StrStr` "T_" (`self.TextureNameNoLegend`) ".png"))))

(fn `UserConstructionScript`
  (bind (_returnvalue_x _returnvalue_y) (break `IntVector` (`GameplayStatics.GetWorldOriginLocation`)))
  (bind _returnvalue (`KismetMathLibrary.SafeDivide` (`self.WorldSizeInUnits`) 100.0))
  (bind _returnvalue_2 (`KismetMathLibrary.SafeDivide` (`self.WorldSizeInUnits`) 100.0))
  (`self.K2_SetActorLocation` (`KismetMathLibrary.MakeVector` (`KismetMathLibrary.Conv_IntToDouble` (/ _returnvalue_x 2)) (`KismetMathLibrary.Conv_IntToDouble` (/ _returnvalue_y 2))))
  (set `self.WorldSizeInUnits` (* (`self.WorldSizeInKm`) 100000.0))
  (`SceneComponent.K2_SetRelativeLocation` (`self.CameraLegend`) (`KismetMathLibrary.MakeVector` 0.0 0.0 (`self.WorldSizeInUnits`)) false false)
  (`SceneComponent.K2_SetRelativeLocation` (`self.CameraNoLegend`) (`KismetMathLibrary.MakeVector` 0.0 0.0 (`self.WorldSizeInUnits`)) false false)
  (`SceneComponent.SetRelativeScale3D` (`self.ProjectionPlaneLegend`) (`KismetMathLibrary.MakeVector` _returnvalue_2 _returnvalue_2 1.0))
  (`SceneComponent.SetRelativeScale3D` (`self.ProjectionPlaneNoLegend`) (`KismetMathLibrary.MakeVector` _returnvalue _returnvalue 1.0))
  (if (`self.bCapture`)
    (`self.MapCaptureLegend`)
    (`self.MapCaptureNoLegend`)
    (set `self.bCapture` false)))