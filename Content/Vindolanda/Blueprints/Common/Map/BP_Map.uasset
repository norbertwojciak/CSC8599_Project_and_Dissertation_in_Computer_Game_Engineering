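; BP_Map is a map capture actor that renders the minimap, big map and two world maps, with and without legend.
; On BeginPlay it creates a render target for each capture component, sizes their ortho widths and starts minimap mode.
; UpdateMapStatus toggles between minimap capture with timed tracking of the owner's position and yaw, and capturing the other three maps from world origin.
; UpdateMapObjects adds components to every capture's show-only list.
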(event `self.ReceiveBeginPlay`
  (bind _minimapsize (`self.MinimapSize`))
  (bind _worldmapsize (`self.WorldMapSize`))
  (bind _worldmapsize_2 (`self.WorldMapSize`))
  (bind _bigmapsize (`self.BigMapSize`))
  ;[1 1 1] RT Minimap
  (bind _returnvalue (`KismetRenderingLibrary.CreateRenderTarget2D` _minimapsize _minimapsize))
  (bind _output_get (set `self.RT_Minimap` _returnvalue))
  (set `SceneCaptureComponent2D.TextureTarget` _output_get (`self.MinimapComponent`))
  (set `SceneCaptureComponent2D.OrthoWidth` (* (`self.MinimapMultiplier`) (`/Game/Vindolanda/Blueprints/FunctionLibrary/BP_FunctionLibrary.Get Map Capture Size`)) (`self.MinimapComponent`))
  ;[1 1 1] RT Big Map
  (bind _returnvalue_2 (`KismetRenderingLibrary.CreateRenderTarget2D` _bigmapsize _bigmapsize))
  (bind _output_get_2 (set `self.RT_BigMap` _returnvalue_2))
  (set `SceneCaptureComponent2D.TextureTarget` _output_get_2 (`self.BigMapComponent`))
  (set `SceneCaptureComponent2D.OrthoWidth` (`/Game/Vindolanda/Blueprints/FunctionLibrary/BP_FunctionLibrary.Get Map Capture Size`) (`self.BigMapComponent`))
  ;[1 1 1] RT World Map
  (bind _returnvalue_3 (`KismetRenderingLibrary.CreateRenderTarget2D` _worldmapsize_2 _worldmapsize_2))
  (bind _output_get_3 (set `self.RT_WorldMapLegend` _returnvalue_3))
  (set `SceneCaptureComponent2D.TextureTarget` _output_get_3 (`self.WorldMapLegendComponent`))
  (set `SceneCaptureComponent2D.OrthoWidth` (`/Game/Vindolanda/Blueprints/FunctionLibrary/BP_FunctionLibrary.Get Map Capture Size`) (`self.WorldMapLegendComponent`))
  ;[1 1 1] RT World Map
  (bind _returnvalue_4 (`KismetRenderingLibrary.CreateRenderTarget2D` _worldmapsize _worldmapsize))
  (bind _output_get_4 (set `self.RT_WorldMapNoLegend` _returnvalue_4))
  (set `SceneCaptureComponent2D.TextureTarget` _output_get_4 (`self.WorldMapNoLegendComponent`))
  (set `SceneCaptureComponent2D.OrthoWidth` (`/Game/Vindolanda/Blueprints/FunctionLibrary/BP_FunctionLibrary.Get Map Capture Size`) (`self.WorldMapNoLegendComponent`))
  (`self.UpdateMapStatus` true))

(event `self.ReceiveDestroyed`
  (`KismetRenderingLibrary.ClearRenderTarget2D` (`self.RT_Minimap`))
  (`KismetRenderingLibrary.ClearRenderTarget2D` (`self.RT_BigMap`))
  (`KismetRenderingLibrary.ClearRenderTarget2D` (`self.RT_WorldMapLegend`))
  (`KismetRenderingLibrary.ClearRenderTarget2D` (`self.RT_WorldMapNoLegend`))
  (`KismetSystemLibrary.K2_ClearAndInvalidateTimerHandle` (`self.Trackingtimer`)))

(fn `DestroyMap`
  (`self.K2_DestroyActor`))

(fn `StartTracking`
  (bind _returnvalue (`self.GetOwner`))
  (bind (_returnvalue_x _returnvalue_y _returnvalue_z) (`KismetMathLibrary.BreakVector` (`self.K2_GetActorLocation`)))
  (bind (_returnvalue_x_2 _returnvalue_y_2) (`KismetMathLibrary.BreakVector` (`self.K2_GetActorLocation` _returnvalue)))
  (bind (_returnvalue_roll _returnvalue_pitch _returnvalue_yaw) (`KismetMathLibrary.BreakRotator` (`self.K2_GetActorRotation` _returnvalue)))
  (`self.K2_SetActorLocationAndRotation` (`KismetMathLibrary.MakeVector` _returnvalue_x_2 _returnvalue_y_2 _returnvalue_z) (`KismetMathLibrary.MakeRotator` 0.0 0.0 _returnvalue_yaw)))

(fn `UpdateMapObjects`
  (params (ShowComponent :type "PrimitiveComponent Object Reference"))
  (`SceneCaptureComponent.ShowOnlyComponent` (`self.MinimapComponent`) (`local.ShowComponent`))
  (`SceneCaptureComponent.ShowOnlyComponent` (`self.BigMapComponent`) (`local.ShowComponent`))
  (`SceneCaptureComponent.ShowOnlyComponent` (`self.WorldMapLegendComponent`) (`local.ShowComponent`))
  (`SceneCaptureComponent.ShowOnlyComponent` (`self.WorldMapNoLegendComponent`) (`local.ShowComponent`)))

(fn `UpdateMapStatus`
  (params (bMinimap :type Boolean) (bBigMap :type Boolean) (bWorldMapLegend :type Boolean) (bWorldMapNoLegend :type Boolean))
  (bind (_returnvalue_x _returnvalue_y) (break `IntVector` (`GameplayStatics.GetWorldOriginLocation`)))
  (bind (_returnvalue_x_2 _returnvalue_y_2 _returnvalue_z) (`KismetMathLibrary.BreakVector` (`self.K2_GetActorLocation`)))
  (if bMinimap
    (bind _returnvalue (`KismetSystemLibrary.K2_SetTimerDelegate` (`|CreateDelegate` :!event `StartTracking`) 0.4 true))
    (set `self.Trackingtimer` _returnvalue)
    (set `SceneCaptureComponent.bCaptureEveryFrame` true (`self.MinimapComponent`))
    (set `SceneCaptureComponent.bCaptureEveryFrame` false (`self.BigMapComponent`))
    (set `SceneCaptureComponent.bCaptureEveryFrame` false (`self.WorldMapLegendComponent`))
    (set `SceneCaptureComponent.bCaptureEveryFrame` false (`self.WorldMapNoLegendComponent`))
    (else
      (`self.K2_SetActorLocationAndRotation` (`KismetMathLibrary.MakeVector` (`KismetMathLibrary.Conv_IntToDouble` _returnvalue_x) (`KismetMathLibrary.Conv_IntToDouble` _returnvalue_y) _returnvalue_z) (`KismetMathLibrary.MakeRotator` 0.0))
      (`KismetSystemLibrary.K2_ClearAndInvalidateTimerHandle` (`self.Trackingtimer`))
      (set `SceneCaptureComponent.bCaptureEveryFrame` false (`self.MinimapComponent`))
      (set `SceneCaptureComponent.bCaptureEveryFrame` true (`self.BigMapComponent`))
      (set `SceneCaptureComponent.bCaptureEveryFrame` true (`self.WorldMapLegendComponent`))
      (set `SceneCaptureComponent.bCaptureEveryFrame` true (`self.WorldMapNoLegendComponent`)))))

(fn `UserConstructionScript`)