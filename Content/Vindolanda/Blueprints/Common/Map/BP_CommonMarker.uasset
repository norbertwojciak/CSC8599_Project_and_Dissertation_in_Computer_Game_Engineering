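; BP_CommonMarker is a map marker actor that shows a textured plane and has a matching map widget.
; Its construction script reads a data table row to set plane height and scale, and BeginPlay applies the row's texture through a dynamic material.
; A timer waits for the player character, then registers the plane and requests the widget through message calls.
; A looping timer then aligns the plane to player yaw in minimap mode, otherwise fixing its rotation.
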(event `CheckPlayerAndProceed`
  (`/Engine/EditorBlueprintResources/StandardMacros.IsValid` (`GameplayStatics.GetPlayerCharacter` 0)
    (:`Is Valid`
      (`KismetSystemLibrary.K2_ClearAndInvalidateTimerHandle` (`self.CheckPlayerTimer`))
      (message `/Game/Vindolanda/Blueprints/Core/BPI_Player_Character.UpdatePlayerMap` (`GameplayStatics.GetPlayerCharacter` 0) (`self.MarkerPlane`))
      (bind _minimapsizeinunits (message `/Game/Vindolanda/Blueprints/Core/BPI_Player_Character.GetMinimapData` (`GameplayStatics.GetPlayerCharacter` 0)))
      (set `self.MinimapSizeInUnits` _minimapsizeinunits)
      (message `/Game/Vindolanda/Blueprints/Core/BPI_Player_Character.CreateMapMarkerWidget` (`GameplayStatics.GetPlayerController` 0) (`self.MarkerData`) (`self.K2_GetActorLocation`) (`self.MinimapSizeInUnits`))
      (bind _returnvalue (`KismetSystemLibrary.K2_SetTimerDelegate` (`|CreateDelegate` :!event `UpdateRotation`) 0.04 true))
      (set `self.UpdateRotationTimer` _returnvalue))))

(event `self.ReceiveBeginPlay`
  (bind _returnvalue (`PrimitiveComponent.CreateDynamicMaterialInstance` (`self.MarkerPlane`) 0 "/Game/Vindolanda/Materials/Map/M_CommonMarker.M_CommonMarker" "None"))
  (set `self.MID_CommonMarker` _returnvalue)
  (`MaterialInstanceDynamic.SetTextureParameterValue` (`self.MID_CommonMarker`) "Texture" (`.Texture_2_9E2E98EC470F051F97994FA934508446` (break `/Game/Vindolanda/Blueprints/Structures/Map/FCommonMarker` (`self.MarkerStructure`))))
  (bind _returnvalue_2 (`KismetSystemLibrary.K2_SetTimerDelegate` (`|CreateDelegate` :!event `CheckPlayerAndProceed`) 0.2 true))
  (set `self.CheckPlayerTimer` _returnvalue_2))

(event `UpdateRotation`
  (bind (_returnvalue_roll _returnvalue_pitch _returnvalue_yaw) (`KismetMathLibrary.BreakRotator` (`self.K2_GetActorRotation` (`GameplayStatics.GetPlayerCharacter` 0))))
  (bind (_minimapsizeinunits _bminimap) (message `/Game/Vindolanda/Blueprints/Core/BPI_Player_Character.GetMinimapData` (`GameplayStatics.GetPlayerCharacter` 0)))
  (set `self.bMinimap` _bminimap)
  (if (not (`self.bMinimap`))
    (`SceneComponent.K2_SetRelativeRotation` (`self.MarkerPlane`) (struct :`Yaw` 90.0) false false)
    (else
      (`SceneComponent.K2_SetRelativeRotation` (`self.MarkerPlane`) (`KismetMathLibrary.MakeRotator` 0.0 0.0 (+ _returnvalue_yaw 90.0)) false false))))

(fn `UnpackDataAndProceed`
  (bind (_returnvalue_x _returnvalue_y) (`KismetMathLibrary.BreakVector` (`self.K2_GetActorLocation`)))
  (bind (_datatable _rowname) (break `DataTableRowHandle` (`self.MarkerData`)))
  (bind (_size_x _size_y) (`KismetMathLibrary.BreakVector2D` (break `/Game/Vindolanda/Blueprints/Structures/Map/FCommonMarker` (`self.MarkerStructure`))))
  (bind _returnvalue (`|GetDataTableRow` _datatable _rowname)
    (:`then`
      (set `self.MarkerStructure` _returnvalue)
      (`self.K2_SetActorLocation` (`KismetMathLibrary.MakeVector` _returnvalue_x _returnvalue_y))
      (`SceneComponent.K2_SetRelativeLocation` (`self.MarkerPlane`) (`KismetMathLibrary.MakeVector` 0.0 0.0 (`.Offset_8_B5AF762B462A81D0552C9F838406EA21` (break `/Game/Vindolanda/Blueprints/Structures/Map/FCommonMarker` (`self.MarkerStructure`)))) false false)
      (`SceneComponent.SetRelativeScale3D` (`self.MarkerPlane`) (`KismetMathLibrary.MakeVector` _size_x _size_y)))))

(fn `UserConstructionScript`
  (`self.UnpackDataAndProceed`)
  (if (`self.bUpdate`)
    (`self.UnpackDataAndProceed`)
    (set `self.bUpdate` false)))