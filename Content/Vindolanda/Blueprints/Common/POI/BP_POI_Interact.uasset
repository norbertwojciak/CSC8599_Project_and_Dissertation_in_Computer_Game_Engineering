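; BP_POI_Interact is an interactable point of interest that shows descriptive text with its own camera view.
; On interaction it pauses backpack and game menu via the game controller, opens the player's description widget and blends the view to itself.
; It also notifies the player's quest component and plays data-table dialogue with subtitles when valid.
; Closing the widget blends back to the player and clears both pause flags.
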(event `self.TopButtonInteraction`
  (set `/Game/TPSAT/Blueprints/Core/BP_StoryAdv_GameController.BackpackPausePOI` true (`/Game/TPSAT/Blueprints/Core/BP_StoryAdv_FunctionLibrary.GetGameController`))
  (set `/Game/TPSAT/Blueprints/Core/BP_StoryAdv_GameController.GameMenuPausePOI` true (`/Game/TPSAT/Blueprints/Core/BP_StoryAdv_FunctionLibrary.GetGameController`))
  (message `/Game/Vindolanda/Blueprints/Common/InteractionSystem/BPI_InteractionSystem.AddDescriptionWidgetInteract` (`GameplayStatics.GetPlayerCharacter` 0) self null (`self.Text_0`) (`self.DelayBetweenLetters_0`))
  (`PlayerController.SetViewTargetWithBlend` (`GameplayStatics.GetPlayerController` 0) self (`self.BlendInTime_0`) "VTBlend_Linear" 0.0 false)
  (`/Game/Vindolanda/Blueprints/Common/BP_QuestComponent.OnQuestItemIneracted` (`self.GetComponentByClass` (`GameplayStatics.GetPlayerCharacter` 0) "/Game/Vindolanda/Blueprints/Common/BP_QuestComponent.BP_QuestComponent_C") "NewEnumerator3" (`GameplayStatics.GetObjectClass` self))
  (bind (_dialogue_waves _subtitles _validdata) (`/Game/TPSAT/Blueprints/Core/BP_StoryAdv_FunctionLibrary.GetDialogueDataFromTable` (`self.DialogueRow`)))
  (if _validdata
    (`/Game/TPSAT/Blueprints/Core/BP_StoryAdv_GameController.PlayPlayerDialogue` (`self.GameControllerInstance`) _dialogue_waves _subtitles)))

(event `/Game/Vindolanda/Blueprints/Common/InteractionSystem/BPI_InteractionSystem.DestroyDescriptionWidgetInteract`
  (`PlayerController.SetViewTargetWithBlend` (`GameplayStatics.GetPlayerController` 0) (`GameplayStatics.GetPlayerCharacter` 0) (`self.BlendOutTime_0`) "VTBlend_Linear" 0.0 false)
  (set `/Game/TPSAT/Blueprints/Core/BP_StoryAdv_GameController.BackpackPausePOI` false (`/Game/TPSAT/Blueprints/Core/BP_StoryAdv_FunctionLibrary.GetGameController`))
  (set `/Game/TPSAT/Blueprints/Core/BP_StoryAdv_GameController.GameMenuPausePOI` false (`/Game/TPSAT/Blueprints/Core/BP_StoryAdv_FunctionLibrary.GetGameController`)))

(fn `UserConstructionScript`)