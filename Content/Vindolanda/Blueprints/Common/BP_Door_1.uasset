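; BP_Door_1 is an interactable door that the player swings open and shut with the Interact input.
; A box overlap by any Character enables input, shows a prompt widget and opens a gate; leaving reverses all three.
; Interact pulses IsPressed for 0.3 seconds, then a FlipFlop plays or reverses one timeline driving door yaw.
; A separate closing timeline is disconnected, so IsDoorClosed is never set true here.
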(event `InputAction|Interact` :consume false
  (params (Key :type "Key Structure"))
  (:`Pressed`
    (set `self.IsPressed` true)
    (`KismetSystemLibrary.Delay` 0.3)
    (set `self.IsPressed` false)
    (`/Engine/EditorBlueprintResources/StandardMacros.Gate` true :!label _label
      (:`Exit`
        (`/Engine/EditorBlueprintResources/StandardMacros.FlipFlop`
          (:`A`
            ;[1 1 1] Open door
            (bind (_direction _doorrotationz) (`Timeline|Timeline_1` :!label _label_2)
              (:`Update`
                (`SceneComponent.K2_SetRelativeRotation` (`self.Door`) (`KismetMathLibrary.MakeRotator` 0.0 0.0 _doorrotationz) false false))
              (:`Finished`
                (set `self.isDoorClosed` false))))
          (:`B`
            (goto _label_2 :!via `Reverse`)))))))

(event `self.Box.OnComponentBeginOverlap`
  (params (OverlappedComponent :type "PrimitiveComponent Object Reference") (OtherActor :type "Actor Object Reference") (OtherComp :type "PrimitiveComponent Object Reference") (OtherBodyIndex :type Integer) (bFromSweep :type Boolean) (SweepResult :type "HitResult Structure (by ref)"))
  ;[1 1 1] Check if the character is close enough
  (cast `Character` OtherActor)
  (`self.EnableInput` (`GameplayStatics.GetPlayerController` 0))
  ;[1 1 1] Add and remove from screen
  (bind _returnvalue (`|CreateWidget` "/Game/Vindolanda/GUI/Interact_Prompt_Widget.Interact_Prompt_Widget_C"))
  (`UserWidget.AddToViewport` _returnvalue 0)
  (goto _label :!via `Open`))

(event `self.Box.OnComponentEndOverlap`
  (params (OverlappedComponent :type "PrimitiveComponent Object Reference") (OtherActor :type "Actor Object Reference") (OtherComp :type "PrimitiveComponent Object Reference") (OtherBodyIndex :type Integer))
  ;[1 1 1] Check if the character is close enough
  (cast `Character` OtherActor)
  (`self.DisableInput` (`GameplayStatics.GetPlayerController` 0))
  ;[1 1 1] Add and remove from screen
  (`Widget.RemoveFromParent` (stale `self.Box.OnComponentBeginOverlap` _returnvalue))
  (goto _label :!via `Close`))

(fn `UserConstructionScript`)