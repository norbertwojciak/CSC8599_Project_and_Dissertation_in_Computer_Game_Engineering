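; Player start actor that spawns the story adventure character on BeginPlay and has player controller 0 possess it.
; Outside Editor mode it loads save data, restoring the current level's saved transform and stamina, or spawning at its own transform when none exists.
; Without a saved transform, NewScenario selects default stamina over saved stamina.
; The Editor flag skips loading entirely and spawns at the actor with its configured values.
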(event `self.ReceiveBeginPlay`
  (bind (_value _returnvalue) (`BlueprintMapLibrary.Map_Find` (`.LevelsTransform_4_AEB1F54C4608642AB364BFBE09048B0B` (break `/Game/Vindolanda/Blueprints/Structures/GameDataChildren/FLevelData` (`.Level_5_041A39A5467F999E49405D8CEBDCB32A` (break `/Game/Vindolanda/Blueprints/Structures/GameDataChildren/FGameData` (`self.GameData`))))) (`self.CurrentLevel`)))
  (if (not (`self.bEditor`))
    (bind _gamedata (`/Game/TPSAT/Blueprints/Core/BP_StoryAdv_GameInstance.Load Game Data from Save Game Slot` (`/Game/TPSAT/Blueprints/Core/BP_StoryAdv_FunctionLibrary.GetStoryAdvGameInstance`)))
    (set `self.GameData` _gamedata)
    (bind _returnvalue_2 (`GameplayStatics.GetCurrentLevelName` true))
    (set `self.CurrentLevel` _returnvalue_2)
    (if _returnvalue
      (set `self.SpawnTransform` _value)
      (bind _returnvalue_3 (`|SpawnActorFromClass` "/Game/TPSAT/Blueprints/Character/BP_StoryAdv_Character.BP_StoryAdv_Character_C" (`self.SpawnTransform`) "Undefined" "OverrideRootScale" null 500.0 250.0 (`self.QuestDB`) (`.Stamina_5_8D6AC9944F1B4B555B649CB17B1AFA99` (break `/Game/Vindolanda/Blueprints/Structures/GameDataChildren/FPlayerData` (`.Player_2_4534EC8D441797AA8F2C708F42772B13` (break `/Game/Vindolanda/Blueprints/Structures/GameDataChildren/FGameData` (`self.GameData`))))) null))
      (set `self.Playercharacter` _returnvalue_3)
      (`Controller.Possess` (`GameplayStatics.GetPlayerController` 0) (`self.Playercharacter`))
      (else
        (set `self.SpawnTransform` (`self.GetTransform`))
        (if (`self.bNewScenario`)
          (bind _returnvalue_4 (`|SpawnActorFromClass` "/Game/TPSAT/Blueprints/Character/BP_StoryAdv_Character.BP_StoryAdv_Character_C" (`self.SpawnTransform`) "Undefined" "OverrideRootScale" null (`self.SprintSpeed`) (`self.WalkSpeed`) (`self.QuestDB`) (`self.Stamina`) null))
          (set `self.Playercharacter` _returnvalue_4)
          (else
            (bind _returnvalue_5 (`|SpawnActorFromClass` "/Game/TPSAT/Blueprints/Character/BP_StoryAdv_Character.BP_StoryAdv_Character_C" (`self.SpawnTransform`) "Undefined" "OverrideRootScale" null (`self.SprintSpeed`) (`self.WalkSpeed`) (`self.QuestDB`) (`.Stamina_5_8D6AC9944F1B4B555B649CB17B1AFA99` (break `/Game/Vindolanda/Blueprints/Structures/GameDataChildren/FPlayerData` (`.Player_2_4534EC8D441797AA8F2C708F42772B13` (break `/Game/Vindolanda/Blueprints/Structures/GameDataChildren/FGameData` (`self.GameData`))))) null))
            (set `self.Playercharacter` _returnvalue_5)))
        (`Controller.Possess` (`GameplayStatics.GetPlayerController` 0) (`self.Playercharacter`))))
    (else
      (bind _returnvalue_6 (`|SpawnActorFromClass` "/Game/TPSAT/Blueprints/Character/BP_StoryAdv_Character.BP_StoryAdv_Character_C" (`self.GetTransform`) "Undefined" "OverrideRootScale" null (`self.SprintSpeed`) (`self.WalkSpeed`) (`self.QuestDB`) (`self.Stamina`) null))
      (set `self.Playercharacter` _returnvalue_6)
      (`Controller.Possess` (`GameplayStatics.GetPlayerController` 0) (`self.Playercharacter`)))))

(fn `UserConstructionScript`)