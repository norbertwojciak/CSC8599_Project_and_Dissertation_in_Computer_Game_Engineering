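; Player controller for Vindolanda that owns the quest HUD and map HUD widgets.
; Events create and remove both widgets, and forward render-target updates and marker creation to the map widget.
; HUD toggle, enable and disable events show or hide the quest widget, set GamePaused and call ToggleWorldMapMessage on the player character.
; GetQuestWidget exposes the quest widget, while GetMinimapData and GetPlayerData are placeholder stubs.
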(event `/Game/Vindolanda/Blueprints/Core/BPI_QuestSystem.CreateQuestWidget`
  ;[0 0.7379 1] Add HUD Quest Widget
  (bind _returnvalue (`|CreateWidget` "/Game/Vindolanda/GUI/HUD_Quest/HUD_Quest.HUD_Quest_C" null null))
  (bind _output_get (set `self.GUI_Quest` _returnvalue))
  (`UserWidget.AddToViewport` _output_get 100))

(event `/Game/Vindolanda/Blueprints/Core/BPI_QuestSystem.DestroyQuestWidget`
  ;[0 0.7379 1] Remove HUD Quest Widget
  (`/Engine/EditorBlueprintResources/StandardMacros.IsValid` (`self.GUI_Quest`)
    (:`Is Valid`
      (`Widget.RemoveFromParent` (`self.GUI_Quest`))
      (set `self.GUI_Quest` null))))

(event `/Game/Vindolanda/Blueprints/Core/BPI_Player_Character.ToggleHUD`
  ;[1 1 1] Toggle HUD
  (`/Engine/EditorBlueprintResources/StandardMacros.FlipFlop`
    (:`A`
      (set `self.GamePaused` false)
      (`Widget.RemoveFromParent` (`self.GUI_Quest`))
      (message `/Game/Vindolanda/Blueprints/Core/BPI_Player_Character.ToggleWorldMap` (`GameplayStatics.GetPlayerCharacter` 0) false false false false))
    (:`B`
      (set `self.GamePaused` true)
      (`UserWidget.AddToViewport` (`self.GUI_Quest`) 0)
      (message `/Game/Vindolanda/Blueprints/Core/BPI_Player_Character.ToggleWorldMap` (`GameplayStatics.GetPlayerCharacter` 0) true false false false))))

(event `/Game/Vindolanda/Blueprints/Core/BPI_Player_Character.DisableHUD`
  (set `self.GamePaused` false)
  (`Widget.RemoveFromParent` (`self.GUI_Quest`))
  (message `/Game/Vindolanda/Blueprints/Core/BPI_Player_Character.ToggleWorldMap` (`GameplayStatics.GetPlayerCharacter` 0) false false false false))

(event `/Game/Vindolanda/Blueprints/Core/BPI_Player_Character.EnableHUD`
  (set `self.GamePaused` true)
  (`UserWidget.AddToViewport` (`self.GUI_Quest`) 0)
  (message `/Game/Vindolanda/Blueprints/Core/BPI_Player_Character.ToggleWorldMap` (`GameplayStatics.GetPlayerCharacter` 0) true false false false))

(event `/Game/Vindolanda/Blueprints/Core/BPI_Player_Character.CreateMapWidget`
  (params (RT_Minimap :type "TextureRenderTarget2D Object Reference") (RT_BigMap :type "TextureRenderTarget2D Object Reference") (RT_WorldMapLegend :type "TextureRenderTarget2D Object Reference") (RT_WorldMapNoLegend :type "TextureRenderTarget2D Object Reference"))
  (bind _returnvalue (`|CreateWidget` "/Game/Vindolanda/GUI/HUD_Map/HUD_Map.HUD_Map_C" null RT_Minimap RT_BigMap RT_WorldMapLegend RT_WorldMapNoLegend))
  (bind _output_get (set `self.GUI_Map` _returnvalue))
  (`UserWidget.AddToViewport` _output_get 1000))

(event `/Game/Vindolanda/Blueprints/Core/BPI_Player_Character.DestroyMapWidget`
  (`/Engine/EditorBlueprintResources/StandardMacros.IsValid` (`self.GUI_Map`)
    (:`Is Valid`
      (`Widget.RemoveFromParent` (`self.GUI_Map`))
      (set `self.GUI_Map` null))))

(event `/Game/Vindolanda/Blueprints/Core/BPI_Player_Character.UpdateMapWidget`
  (params (Minimap :type Boolean) (BigMap :type Boolean) (WorldMapLegend :type Boolean) (WorldMapNoLegend :type Boolean))
  (`/Engine/EditorBlueprintResources/StandardMacros.IsValid` (`self.GUI_Map`)
    (:`Is Valid`
      (`/Game/Vindolanda/GUI/HUD_Map/HUD_Map.Update Map` (`self.GUI_Map`) Minimap BigMap WorldMapLegend WorldMapNoLegend))))

(event `/Game/Vindolanda/Blueprints/Core/BPI_Player_Character.CreateMapMarkerWidget`
  (params (MarkerData :type "DataTableRowHandle Structure") (Location :type "Vector Structure") (MinimapSizeInUnits :type "Float (single-precision)"))
  (`/Engine/EditorBlueprintResources/StandardMacros.IsValid` (`self.GUI_Map`)
    (:`Is Valid`
      (`/Game/Vindolanda/GUI/HUD_Map/HUD_Map.CreateMapMarker` (`self.GUI_Map`) MarkerData Location MinimapSizeInUnits))))

(fn `GetMinimapData`
  (returns (MinimapSizeInUnits :type "Float (double-precision)") (bMinimap :type Boolean))
  (return 0.0 false))

(fn `GetPlayerData`
  (returns (PlayerData :type "/Game/Vindolanda/Blueprints/Structures/GameDataChildren/FPlayerData Structure")))

(fn `GetQuestWidget`
  (returns (GUI_Quest :type "/Game/Vindolanda/GUI/HUD_Quest/HUD_Quest Object Reference"))
  (return (`self.GUI_Quest`)))

(fn `UserConstructionScript`)